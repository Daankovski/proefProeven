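; Battery placement socket that snaps a BP_Placeable_Battery into place and flags itself Finished.
; On overlap, a DoOnce calls the player's PickupEvent, disables battery physics, attaches it and turns the light and dynamic button material green.
; End overlap turns both red and resets the DoOnce, but leaves Finished set.
; The light functions ignore their index, and the ForEachLoopWithDelay macro is unused here.
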(event `self.ReceiveBeginPlay`)

(event `self.Btn_1_Collider.OnComponentBeginOverlap`
  (params (OverlappedComponent :type "PrimitiveComponent Object Reference") (OtherActor :type "Actor Object Reference") (OtherComp :type "PrimitiveComponent Object Reference") (OtherBodyIndex :type Integer) (bFromSweep :type Boolean) (SweepResult :type "HitResult Structure (by ref)"))
  (bind _asbp_placeable_battery (cast `/Game/Blueprints/BP_Placeable_Battery` OtherActor))
  (`/Engine/EditorBlueprintResources/StandardMacros.DoOnce` false :!label _label
    (:`Completed`
      (bind _output_get (set `self.TmpObject` _asbp_placeable_battery))
      (bind _asfirst_person_character (cast `/Game/FirstPersonBP/Blueprints/FirstPersonCharacter` (`GameplayStatics.GetPlayerPawn` 0)))
      (`/Game/FirstPersonBP/Blueprints/FirstPersonCharacter.PickupEvent` _asfirst_person_character)
      (`PrimitiveComponent.SetSimulatePhysics` (`/Game/Blueprints/BP_Placeable_Battery.StaticMesh` _output_get) false)
      (`self.K2_AttachToComponent` _output_get (`self.Attach`) "None" "SnapToTarget" "SnapToTarget" "KeepWorld" false)
      (`self.ActivateLight` 0)
      (set `self.Finished` true))))

(event `self.Btn_1_Collider.OnComponentEndOverlap`
  (params (OverlappedComponent :type "PrimitiveComponent Object Reference") (OtherActor :type "Actor Object Reference") (OtherComp :type "PrimitiveComponent Object Reference") (OtherBodyIndex :type Integer))
  (cast `/Game/Blueprints/BP_Placeable_Battery` OtherActor)
  (`self.DeactivateLights` 0)
  (goto _label :!via `Reset`))

(fn `ActivateLight`
  (params (Light :type Integer))
  (bind _btn_1_light (`self.Btn_1_Light`))
  (`LightComponent.SetIntensity` _btn_1_light 5000.0)
  (`LightComponent.SetLightColor` _btn_1_light (struct :`G` 1.0 :`A` 1.0) true)
  (`MaterialInstanceDynamic.SetVectorParameterValue` (`self.BTN_1_MAT`) "Color" (struct :`G` 1.0 :`A` 1.0)))

(fn `DeactivateLights`
  (params (Lights :type Integer))
  (bind _btn_1_light (`self.Btn_1_Light`))
  (`LightComponent.SetIntensity` _btn_1_light 5000.0)
  (`LightComponent.SetLightColor` _btn_1_light (struct :`R` 1.0 :`A` 1.0) true)
  (`MaterialInstanceDynamic.SetVectorParameterValue` (`self.BTN_1_MAT`) "Color" (struct :`R` 1.0 :`A` 1.0)))

(fn `UserConstructionScript`
  (`|ExecutionSequence`
    (:`then_0`
      (bind _returnvalue (`PrimitiveComponent.CreateDynamicMaterialInstance` (`self.Button_01`) 0 "/Game/Materials/M_SimonButton.M_SimonButton"))
      (set `self.BTN_1_MAT` _returnvalue))
    (:`then_1`
      (`self.DeactivateLights` 0)
      (`self.DeactivateLights` 1)
      (`self.DeactivateLights` 2)
      (`self.DeactivateLights` 3))))