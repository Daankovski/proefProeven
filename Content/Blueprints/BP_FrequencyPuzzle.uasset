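; Frequency-matching puzzle actor that shows a target and a player frequency on a screen through a dynamic material.
; The construction script randomizes the target, sets a fixed player starting value, and passes both to M_Frequency as vector parameters, packing each frequency into a LinearColor.
; Tick compares all four channels with a tiny tolerance and prints WIN on a match.
; Nothing in this graph changes the player frequency.
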(event `self.ReceiveBeginPlay`)

(event `self.ReceiveTick`
  (params (DeltaSeconds :type "Float (single-precision)"))
  (bind (_basefrequency_r _basefrequency_g _basefrequency_b _basefrequency_a) (break `LinearColor` (`self.BaseFrequency`)))
  (bind (_playerfrequency_r _playerfrequency_g _playerfrequency_b _playerfrequency_a) (break `LinearColor` (`self.PlayerFrequency`)))
  (if (and (and (`KismetMathLibrary.NearlyEqual_FloatFloat` _basefrequency_r _playerfrequency_r) (`KismetMathLibrary.NearlyEqual_FloatFloat` _basefrequency_g _playerfrequency_g)) (and (`KismetMathLibrary.NearlyEqual_FloatFloat` _basefrequency_b _playerfrequency_b) (`KismetMathLibrary.NearlyEqual_FloatFloat` _basefrequency_a _playerfrequency_a)))
    (`KismetSystemLibrary.PrintString` "WIN")))

(fn `UserConstructionScript`
  (bind _returnvalue (`KismetMathLibrary.RandomFloatInRange` -3.0 -1.0))
  (bind _returnvalue_2 (`PrimitiveComponent.CreateDynamicMaterialInstance` (`self.Screen`) 0 "/Game/Materials/M_Frequency.M_Frequency"))
  (bind _output_get (set `self.M_Frequency` _returnvalue_2))
  (bind _output_get_2 (set `self.BaseFrequency` (make `LinearColor` (`KismetMathLibrary.RandomFloatInRange` -2.0 0.0) (`KismetMathLibrary.RandomFloatInRange` 0.0 2.0) _returnvalue (* _returnvalue -1.0))))
  (`MaterialInstanceDynamic.SetVectorParameterValue` _output_get "Range_1" _output_get_2)
  (bind _output_get_3 (set `self.PlayerFrequency` (make `LinearColor` -1.0 1.0 -2.0 2.0)))
  (`MaterialInstanceDynamic.SetVectorParameterValue` (`self.M_Frequency`) "Range_2" _output_get_3))