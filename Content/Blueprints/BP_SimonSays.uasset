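; Simon Says memory game actor with four colored buttons, lit through point-light intensity and dynamic material colors.
; BeginPlay and the construction script flash an intro; SimonTurn appends a random button and replays the sequence with delays.
; FirstPersonCharacter overlaps, gated by DoOnce until exit, feed ActivateButton, which checks input outside Simon's turn.
; ActivateButton is SimonTurn's only caller: a completed sequence extends it, a mistake clears it and restarts.
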(event `StartSimon`
  (`self.ActivateLight` 0)
  (`KismetSystemLibrary.Delay` 0.2)
  (`self.ActivateLight` 1)
  (`KismetSystemLibrary.Delay` 0.2)
  (`self.ActivateLight` 2)
  (`KismetSystemLibrary.Delay` 0.2)
  (`self.ActivateLight` 3)
  (`KismetSystemLibrary.Delay` 1.0)
  (`self.DeactivateLights`))

(event `SimonTurn`
  (set `self.IsSimonTurn` true)
  (`KismetArrayLibrary.Array_Add` (`self.ButtonSequence`) (`KismetMathLibrary.RandomInteger` 4))
  (`self.ActivateLight` (`|GetArrayItem` (`self.ButtonSequence`) (`self.ArrayIndex_Simon`)) :!label _label)
  (`KismetSystemLibrary.Delay` 0.5)
  (`self.DeactivateLights`)
  (bind _result (`/Engine/EditorBlueprintResources/StandardMacros.IncrementInt` (`self.ArrayIndex_Simon`))
    (:`  `
      (if (== _result (`KismetArrayLibrary.Array_Length` (`self.ButtonSequence`)))
        (set `self.ArrayIndex_Simon` 0)
        (set `self.IsSimonTurn` false)
        (else
          (`KismetSystemLibrary.Delay` 0.2)
          (goto _label))))))

(event `self.ReceiveBeginPlay`
  (`self.StartSimon`))

(event `self.Btn_1_Collider.OnComponentBeginOverlap`
  (params (OverlappedComponent :type "PrimitiveComponent Object Reference") (OtherActor :type "Actor Object Reference") (OtherComp :type "PrimitiveComponent Object Reference") (OtherBodyIndex :type Integer) (bFromSweep :type Boolean) (SweepResult :type "HitResult Structure (by ref)"))
  (cast `/Game/FirstPersonBP/Blueprints/FirstPersonCharacter` OtherActor)
  (`/Engine/EditorBlueprintResources/StandardMacros.DoOnce` false :!label _label_2
    (:`Completed`
      (`self.ActivateButton` 0))))

(event `ActivateButton`
  (params (Button :type Integer))
  (if (`self.IsSimonTurn`)
    _
    (elif (== Button (`|GetArrayItem` (`self.ButtonSequence`) (`self.ArrayIndex_Player`)))
      (bind _result (`/Engine/EditorBlueprintResources/StandardMacros.IncrementInt` (`self.ArrayIndex_Player`))
        (:`  `
          (if (== _result (`KismetArrayLibrary.Array_Length` (`self.ButtonSequence`)))
            (`KismetSystemLibrary.Delay` 1.0)
            (set `self.ArrayIndex_Player` 0)
            (`self.SimonTurn`))))
      (else
        (set `self.IsSimonTurn` true)
        (`KismetArrayLibrary.Array_Clear` (`self.ButtonSequence`))
        (set `self.ArrayIndex_Player` 0)
        (`KismetSystemLibrary.Delay` 2.0)
        (`self.SimonTurn`)))))

(event `self.Btn_1_Collider.OnComponentEndOverlap`
  (params (OverlappedComponent :type "PrimitiveComponent Object Reference") (OtherActor :type "Actor Object Reference") (OtherComp :type "PrimitiveComponent Object Reference") (OtherBodyIndex :type Integer))
  (goto _label_2 :!via `Reset`))

(event `self.Btn_2_Collider.OnComponentBeginOverlap`
  (params (OverlappedComponent :type "PrimitiveComponent Object Reference") (OtherActor :type "Actor Object Reference") (OtherComp :type "PrimitiveComponent Object Reference") (OtherBodyIndex :type Integer) (bFromSweep :type Boolean) (SweepResult :type "HitResult Structure (by ref)"))
  (cast `/Game/FirstPersonBP/Blueprints/FirstPersonCharacter` OtherActor)
  (`/Engine/EditorBlueprintResources/StandardMacros.DoOnce` false :!label _label_3
    (:`Completed`
      (`self.ActivateButton` 1))))

(event `self.Btn_2_Collider.OnComponentEndOverlap`
  (params (OverlappedComponent :type "PrimitiveComponent Object Reference") (OtherActor :type "Actor Object Reference") (OtherComp :type "PrimitiveComponent Object Reference") (OtherBodyIndex :type Integer))
  (goto _label_3 :!via `Reset`))

(event `self.Btn_3_Collider.OnComponentBeginOverlap`
  (params (OverlappedComponent :type "PrimitiveComponent Object Reference") (OtherActor :type "Actor Object Reference") (OtherComp :type "PrimitiveComponent Object Reference") (OtherBodyIndex :type Integer) (bFromSweep :type Boolean) (SweepResult :type "HitResult Structure (by ref)"))
  (cast `/Game/FirstPersonBP/Blueprints/FirstPersonCharacter` OtherActor)
  (`/Engine/EditorBlueprintResources/StandardMacros.DoOnce` false :!label _label_4
    (:`Completed`
      (`self.ActivateButton` 2))))

(event `self.Btn_3_Collider.OnComponentEndOverlap`
  (params (OverlappedComponent :type "PrimitiveComponent Object Reference") (OtherActor :type "Actor Object Reference") (OtherComp :type "PrimitiveComponent Object Reference") (OtherBodyIndex :type Integer))
  (goto _label_4 :!via `Reset`))

(event `self.Btn_4_Collider.OnComponentBeginOverlap`
  (params (OverlappedComponent :type "PrimitiveComponent Object Reference") (OtherActor :type "Actor Object Reference") (OtherComp :type "PrimitiveComponent Object Reference") (OtherBodyIndex :type Integer) (bFromSweep :type Boolean) (SweepResult :type "HitResult Structure (by ref)"))
  (cast `/Game/FirstPersonBP/Blueprints/FirstPersonCharacter` OtherActor)
  (`/Engine/EditorBlueprintResources/StandardMacros.DoOnce` false :!label _label_5
    (:`Completed`
      (`self.ActivateButton` 3))))

(event `self.Btn_4_Collider.OnComponentEndOverlap`
  (params (OverlappedComponent :type "PrimitiveComponent Object Reference") (OtherActor :type "Actor Object Reference") (OtherComp :type "PrimitiveComponent Object Reference") (OtherBodyIndex :type Integer))
  (goto _label_5 :!via `Reset`))

(fn `ActivateLight`
  (params (Light :type Integer))
  (switch `int` Light
    (:`0`
      (`LightComponent.SetIntensity` (`self.Btn_1_Light`) 5000.0)
      (`MaterialInstanceDynamic.SetVectorParameterValue` (`self.BTN_1_MAT`) "Color" (struct :`R` 1.0 :`A` 1.0)))
    (:`1`
      (`LightComponent.SetIntensity` (`self.Btn_2_Light`) 5000.0)
      (`MaterialInstanceDynamic.SetVectorParameterValue` (`self.BTN_2_MAT`) "Color" (struct :`B` 1.0 :`A` 1.0)))
    (:`2`
      (`LightComponent.SetIntensity` (`self.Btn_3_Light`) 5000.0)
      (`MaterialInstanceDynamic.SetVectorParameterValue` (`self.BTN_3_MAT`) "Color" (struct :`G` 1.0 :`A` 1.0)))
    (:`3`
      (`LightComponent.SetIntensity` (`self.Btn_4_Light`) 5000.0)
      (`MaterialInstanceDynamic.SetVectorParameterValue` (`self.BTN_4_MAT`) "Color" (struct :`R` 1.0 :`G` 1.0 :`A` 1.0)))))

(fn `DeactivateLights`
  (`|ExecutionSequence`
    (:`then_0`
      (`LightComponent.SetIntensity` (`self.Btn_1_Light`) 0.0)
      (`MaterialInstanceDynamic.SetVectorParameterValue` (`self.BTN_1_MAT`) "Color" (struct :`R` 1.0 :`G` 1.0 :`B` 1.0 :`A` 1.0)))
    (:`then_1`
      (`LightComponent.SetIntensity` (`self.Btn_2_Light`) 0.0)
      (`MaterialInstanceDynamic.SetVectorParameterValue` (`self.BTN_2_MAT`) "Color" (struct :`R` 1.0 :`G` 1.0 :`B` 1.0 :`A` 1.0)))
    (:`then_2`
      (`LightComponent.SetIntensity` (`self.Btn_3_Light`) 0.0)
      (`MaterialInstanceDynamic.SetVectorParameterValue` (`self.BTN_3_MAT`) "Color" (struct :`R` 1.0 :`G` 1.0 :`B` 1.0 :`A` 1.0)))
    (:`then_3`
      (`LightComponent.SetIntensity` (`self.Btn_4_Light`) 0.0)
      (`MaterialInstanceDynamic.SetVectorParameterValue` (`self.BTN_4_MAT`) "Color" (struct :`R` 1.0 :`G` 1.0 :`B` 1.0 :`A` 1.0)))))

(fn `UserConstructionScript`
  (`|ExecutionSequence`
    (:`then_0`
      (bind _returnvalue (`PrimitiveComponent.CreateDynamicMaterialInstance` (`self.Button_01`) 0 "/Game/Materials/M_SimonButton.M_SimonButton"))
      (set `self.BTN_1_MAT` _returnvalue))
    (:`then_1`
      (bind _returnvalue_2 (`PrimitiveComponent.CreateDynamicMaterialInstance` (`self.Button_02`) 0 "/Game/Materials/M_SimonButton.M_SimonButton"))
      (set `self.BTN_2_MAT` _returnvalue_2))
    (:`then_2`
      (bind _returnvalue_3 (`PrimitiveComponent.CreateDynamicMaterialInstance` (`self.Button_03`) 0 "/Game/Materials/M_SimonButton.M_SimonButton"))
      (set `self.BTN_3_MAT` _returnvalue_3))
    (:`then_3`
      (bind _returnvalue_4 (`PrimitiveComponent.CreateDynamicMaterialInstance` (`self.Button_04`) 0 "/Game/Materials/M_SimonButton.M_SimonButton"))
      (set `self.BTN_4_MAT` _returnvalue_4))
    (:`then_4`
      (`self.DeactivateLights`))
    (:`then_5`
      (`self.StartSimon`))))