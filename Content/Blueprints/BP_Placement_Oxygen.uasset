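; Oxygen placement puzzle with three slots that accept BP_Placeable_Oxygen items with specific values.
; A valid overlap calls the player's PickupEvent, stops item physics, snaps it to the slot and turns its dynamic-material button and light green.
; Once all three slot flags are set, Finished becomes true.
; End overlap turns the slot red and resets its DoOnce, but leaves the flag set.
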(event `self.ReceiveBeginPlay`)

(event `self.Btn_1_Collider.OnComponentBeginOverlap`
  (params (OverlappedComponent :type "PrimitiveComponent Object Reference") (OtherActor :type "Actor Object Reference") (OtherComp :type "PrimitiveComponent Object Reference") (OtherBodyIndex :type Integer) (bFromSweep :type Boolean) (SweepResult :type "HitResult Structure (by ref)"))
  (bind _asbp_placeable_oxygen (cast `/Game/Blueprints/BP_Placeable_Oxygen` OtherActor))
  (`/Engine/EditorBlueprintResources/StandardMacros.DoOnce` false :!label _label
    (:`Completed`
      (bind _value (`/Game/Blueprints/BP_Placeable_Oxygen.Value` _asbp_placeable_oxygen))
      (if (or (== _value 4) (or (== _value 7) (== _value 8)))
        (bind _output_get (set `self.TmpObject` _asbp_placeable_oxygen))
        (bind _asfirst_person_character (cast `/Game/FirstPersonBP/Blueprints/FirstPersonCharacter` (`GameplayStatics.GetPlayerPawn` 0)))
        (`/Game/FirstPersonBP/Blueprints/FirstPersonCharacter.PickupEvent` _asfirst_person_character)
        (`PrimitiveComponent.SetSimulatePhysics` (`/Game/Blueprints/BP_Placeable_Oxygen.StaticMesh` _output_get) false)
        (`self.K2_AttachToComponent` _output_get (`self.Btn_1_Attach`) "None" "SnapToTarget" "SnapToTarget" "KeepWorld" false)
        (`self.ActivateLight` 0)
        (set `self.Btn1` true)
        (`self.IsFinished`)))))

(event `self.Btn_1_Collider.OnComponentEndOverlap`
  (params (OverlappedComponent :type "PrimitiveComponent Object Reference") (OtherActor :type "Actor Object Reference") (OtherComp :type "PrimitiveComponent Object Reference") (OtherBodyIndex :type Integer))
  (`self.DeactivateLights` 0)
  (goto _label :!via `Reset`))

(event `self.Btn_2_Collider.OnComponentBeginOverlap`
  (params (OverlappedComponent :type "PrimitiveComponent Object Reference") (OtherActor :type "Actor Object Reference") (OtherComp :type "PrimitiveComponent Object Reference") (OtherBodyIndex :type Integer) (bFromSweep :type Boolean) (SweepResult :type "HitResult Structure (by ref)"))
  (bind _asbp_placeable_oxygen (cast `/Game/Blueprints/BP_Placeable_Oxygen` OtherActor))
  (`/Engine/EditorBlueprintResources/StandardMacros.DoOnce` false :!label _label_2
    (:`Completed`
      (bind _value (`/Game/Blueprints/BP_Placeable_Oxygen.Value` _asbp_placeable_oxygen))
      (if (or (== _value 4) (or (== _value 7) (== _value 8)))
        (bind _output_get (set `self.TmpObject` _asbp_placeable_oxygen))
        (bind _asfirst_person_character (cast `/Game/FirstPersonBP/Blueprints/FirstPersonCharacter` (`GameplayStatics.GetPlayerPawn` 0)))
        (`/Game/FirstPersonBP/Blueprints/FirstPersonCharacter.PickupEvent` _asfirst_person_character)
        (`PrimitiveComponent.SetSimulatePhysics` (`/Game/Blueprints/BP_Placeable_Oxygen.StaticMesh` _output_get) false)
        (`self.K2_AttachToComponent` _output_get (`self.Btn_2_Attach`) "None" "SnapToTarget" "SnapToTarget" "KeepWorld" false)
        (`self.ActivateLight` 1)
        (set `self.Btn2` true)
        (`self.IsFinished`)))))

(event `self.Btn_2_Collider.OnComponentEndOverlap`
  (params (OverlappedComponent :type "PrimitiveComponent Object Reference") (OtherActor :type "Actor Object Reference") (OtherComp :type "PrimitiveComponent Object Reference") (OtherBodyIndex :type Integer))
  (`self.DeactivateLights` 1)
  (goto _label_2 :!via `Reset`))

(event `self.Btn_3_Collider.OnComponentBeginOverlap`
  (params (OverlappedComponent :type "PrimitiveComponent Object Reference") (OtherActor :type "Actor Object Reference") (OtherComp :type "PrimitiveComponent Object Reference") (OtherBodyIndex :type Integer) (bFromSweep :type Boolean) (SweepResult :type "HitResult Structure (by ref)"))
  (bind _asbp_placeable_oxygen (cast `/Game/Blueprints/BP_Placeable_Oxygen` OtherActor))
  (`/Engine/EditorBlueprintResources/StandardMacros.DoOnce` false :!label _label_3
    (:`Completed`
      (bind _value (`/Game/Blueprints/BP_Placeable_Oxygen.Value` _asbp_placeable_oxygen))
      (if (or (== _value 4) (or (== _value 7) (== _value 8)))
        (bind _output_get (set `self.TmpObject` _asbp_placeable_oxygen))
        (bind _asfirst_person_character (cast `/Game/FirstPersonBP/Blueprints/FirstPersonCharacter` (`GameplayStatics.GetPlayerPawn` 0)))
        (`/Game/FirstPersonBP/Blueprints/FirstPersonCharacter.PickupEvent` _asfirst_person_character)
        (`PrimitiveComponent.SetSimulatePhysics` (`/Game/Blueprints/BP_Placeable_Oxygen.StaticMesh` _output_get) false)
        (`self.K2_AttachToComponent` _output_get (`self.Btn_3_Attach`) "None" "SnapToTarget" "SnapToTarget" "KeepWorld" false)
        (`self.ActivateLight` 2)
        (set `self.Btn3` true)
        (`self.IsFinished`)))))

(event `self.Btn_3_Collider.OnComponentEndOverlap`
  (params (OverlappedComponent :type "PrimitiveComponent Object Reference") (OtherActor :type "Actor Object Reference") (OtherComp :type "PrimitiveComponent Object Reference") (OtherBodyIndex :type Integer))
  (`self.DeactivateLights` 2)
  (goto _label_3 :!via `Reset`))

(fn `ActivateLight`
  (params (Light :type Integer))
  (bind _btn_1_light (`self.Btn_1_Light`))
  (bind _btn_2_light (`self.Btn_2_Light`))
  (bind _btn_3_light (`self.Btn_3_Light`))
  (switch `int` Light
    (:`0`
      (`LightComponent.SetIntensity` _btn_1_light 5000.0)
      (`LightComponent.SetLightColor` _btn_1_light (struct :`G` 1.0 :`A` 1.0) true)
      (`MaterialInstanceDynamic.SetVectorParameterValue` (`self.BTN_1_MAT`) "Color" (struct :`G` 1.0 :`A` 1.0)))
    (:`1`
      (`LightComponent.SetIntensity` _btn_2_light 5000.0)
      (`LightComponent.SetLightColor` _btn_2_light (struct :`G` 1.0 :`A` 1.0) true)
      (`MaterialInstanceDynamic.SetVectorParameterValue` (`self.BTN_2_MAT`) "Color" (struct :`G` 1.0 :`A` 1.0)))
    (:`2`
      (`LightComponent.SetIntensity` _btn_3_light 5000.0)
      (`LightComponent.SetLightColor` _btn_3_light (struct :`G` 1.0 :`A` 1.0) true)
      (`MaterialInstanceDynamic.SetVectorParameterValue` (`self.BTN_3_MAT`) "Color" (struct :`G` 1.0 :`A` 1.0)))))

(fn `DeactivateLights`
  (params (Lights :type Integer))
  (bind _btn_1_light (`self.Btn_1_Light`))
  (bind _btn_2_light (`self.Btn_2_Light`))
  (bind _btn_3_light (`self.Btn_3_Light`))
  (switch `int` Lights
    (:`0`
      (`LightComponent.SetIntensity` _btn_1_light 5000.0)
      (`LightComponent.SetLightColor` _btn_1_light (struct :`R` 1.0 :`A` 1.0) true)
      (`MaterialInstanceDynamic.SetVectorParameterValue` (`self.BTN_1_MAT`) "Color" (struct :`R` 1.0 :`A` 1.0)))
    (:`1`
      (`LightComponent.SetIntensity` _btn_2_light 5000.0)
      (`LightComponent.SetLightColor` _btn_2_light (struct :`R` 1.0 :`A` 1.0) true)
      (`MaterialInstanceDynamic.SetVectorParameterValue` (`self.BTN_2_MAT`) "Color" (struct :`R` 1.0 :`A` 1.0)))
    (:`2`
      (`LightComponent.SetIntensity` _btn_3_light 5000.0)
      (`LightComponent.SetLightColor` _btn_3_light (struct :`R` 1.0 :`A` 1.0) true)
      (`MaterialInstanceDynamic.SetVectorParameterValue` (`self.BTN_3_MAT`) "Color" (struct :`R` 1.0 :`A` 1.0)))))

(fn `IsFinished`
  (if (and (`self.Btn1`) (and (`self.Btn2`) (`self.Btn3`)))
    (set `self.Finished` true)))

(fn `UserConstructionScript`
  (`|ExecutionSequence`
    (:`then_0`
      (bind _returnvalue (`PrimitiveComponent.CreateDynamicMaterialInstance` (`self.Button_01`) 0 "/Game/Materials/M_SimonButton.M_SimonButton"))
      (set `self.BTN_1_MAT` _returnvalue))
    (:`then_1`
      (bind _returnvalue_2 (`PrimitiveComponent.CreateDynamicMaterialInstance` (`self.Button_02`) 0 "/Game/Materials/M_SimonButton.M_SimonButton"))
      (set `self.BTN_2_MAT` _returnvalue_2))
    (:`then_2`
      (bind _returnvalue_3 (`PrimitiveComponent.CreateDynamicMaterialInstance` (`self.Button_03`) 0 "/Game/Materials/M_SimonButton.M_SimonButton"))
      (set `self.BTN_3_MAT` _returnvalue_3))
    (:`then_3`
      (`self.DeactivateLights` 0)
      (`self.DeactivateLights` 1)
      (`self.DeactivateLights` 2))))