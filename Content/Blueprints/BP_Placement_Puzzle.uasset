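; Placement puzzle actor with four buttons that turn from red to green when a BP_Placeable_Object overlaps their colliders.
; Each overlap, gated by a DoOnce, flags the object as correctly placed; any end overlap resets that button but leaves the flag set.
; Lights and dynamic materials show button state.
; The completion check keeps only the last object's flag, and its success branch is empty.
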(event `self.ReceiveBeginPlay`)

(event `self.Btn_1_Collider.OnComponentBeginOverlap`
  (params (OverlappedComponent :type "PrimitiveComponent Object Reference") (OtherActor :type "Actor Object Reference") (OtherComp :type "PrimitiveComponent Object Reference") (OtherBodyIndex :type Integer) (bFromSweep :type Boolean) (SweepResult :type "HitResult Structure (by ref)"))
  (bind _asbp_placeable_object (cast `/Game/Blueprints/BP_Placeable_Object` OtherActor))
  (`/Engine/EditorBlueprintResources/StandardMacros.DoOnce` false :!label _label
    (:`Completed`
      (set `/Game/Blueprints/BP_Placeable_Object.isPlacedOnCorrectSpot` true _asbp_placeable_object)
      (`self.ActivateLight` 0)
      (`self.CheckIfPuzzleIsComplete`))))

(event `self.Btn_1_Collider.OnComponentEndOverlap`
  (params (OverlappedComponent :type "PrimitiveComponent Object Reference") (OtherActor :type "Actor Object Reference") (OtherComp :type "PrimitiveComponent Object Reference") (OtherBodyIndex :type Integer))
  (`self.DeactivateLights` 0)
  (goto _label :!via `Reset`))

(event `self.Btn_2_Collider.OnComponentBeginOverlap`
  (params (OverlappedComponent :type "PrimitiveComponent Object Reference") (OtherActor :type "Actor Object Reference") (OtherComp :type "PrimitiveComponent Object Reference") (OtherBodyIndex :type Integer) (bFromSweep :type Boolean) (SweepResult :type "HitResult Structure (by ref)"))
  (bind _asbp_placeable_object (cast `/Game/Blueprints/BP_Placeable_Object` OtherActor))
  (`/Engine/EditorBlueprintResources/StandardMacros.DoOnce` false :!label _label_2
    (:`Completed`
      (set `/Game/Blueprints/BP_Placeable_Object.isPlacedOnCorrectSpot` true _asbp_placeable_object)
      (`self.ActivateLight` 1)
      (`self.CheckIfPuzzleIsComplete`))))

(event `self.Btn_2_Collider.OnComponentEndOverlap`
  (params (OverlappedComponent :type "PrimitiveComponent Object Reference") (OtherActor :type "Actor Object Reference") (OtherComp :type "PrimitiveComponent Object Reference") (OtherBodyIndex :type Integer))
  (`self.DeactivateLights` 1)
  (goto _label_2 :!via `Reset`))

(event `self.Btn_3_Collider.OnComponentBeginOverlap`
  (params (OverlappedComponent :type "PrimitiveComponent Object Reference") (OtherActor :type "Actor Object Reference") (OtherComp :type "PrimitiveComponent Object Reference") (OtherBodyIndex :type Integer) (bFromSweep :type Boolean) (SweepResult :type "HitResult Structure (by ref)"))
  (bind _asbp_placeable_object (cast `/Game/Blueprints/BP_Placeable_Object` OtherActor))
  (`/Engine/EditorBlueprintResources/StandardMacros.DoOnce` false :!label _label_3
    (:`Completed`
      (set `/Game/Blueprints/BP_Placeable_Object.isPlacedOnCorrectSpot` true _asbp_placeable_object)
      (`self.ActivateLight` 2)
      (`self.CheckIfPuzzleIsComplete`))))

(event `self.Btn_3_Collider.OnComponentEndOverlap`
  (params (OverlappedComponent :type "PrimitiveComponent Object Reference") (OtherActor :type "Actor Object Reference") (OtherComp :type "PrimitiveComponent Object Reference") (OtherBodyIndex :type Integer))
  (`self.DeactivateLights` 2)
  (goto _label_3 :!via `Reset`))

(event `self.Btn_4_Collider.OnComponentBeginOverlap`
  (params (OverlappedComponent :type "PrimitiveComponent Object Reference") (OtherActor :type "Actor Object Reference") (OtherComp :type "PrimitiveComponent Object Reference") (OtherBodyIndex :type Integer) (bFromSweep :type Boolean) (SweepResult :type "HitResult Structure (by ref)"))
  (bind _asbp_placeable_object (cast `/Game/Blueprints/BP_Placeable_Object` OtherActor))
  (`/Engine/EditorBlueprintResources/StandardMacros.DoOnce` false :!label _label_4
    (:`Completed`
      (set `/Game/Blueprints/BP_Placeable_Object.isPlacedOnCorrectSpot` true _asbp_placeable_object)
      (`self.ActivateLight` 3)
      (`self.CheckIfPuzzleIsComplete`))))

(event `self.Btn_4_Collider.OnComponentEndOverlap`
  (params (OverlappedComponent :type "PrimitiveComponent Object Reference") (OtherActor :type "Actor Object Reference") (OtherComp :type "PrimitiveComponent Object Reference") (OtherBodyIndex :type Integer))
  (`self.DeactivateLights` 3)
  (goto _label_4 :!via `Reset`))

(fn `ActivateLight`
  (params (Light :type Integer))
  (bind _btn_1_light (`self.Btn_1_Light`))
  (bind _btn_2_light (`self.Btn_2_Light`))
  (bind _btn_3_light (`self.Btn_3_Light`))
  (bind _btn_4_light (`self.Btn_4_Light`))
  (switch `int` Light
    (:`0`
      (`LightComponent.SetIntensity` _btn_1_light 5000.0)
      (`LightComponent.SetLightColor` _btn_1_light (struct :`G` 1.0 :`A` 1.0) true)
      (`MaterialInstanceDynamic.SetVectorParameterValue` (`self.BTN_1_MAT`) "Color" (struct :`G` 1.0 :`A` 1.0)))
    (:`1`
      (`LightComponent.SetIntensity` _btn_2_light 5000.0)
      (`LightComponent.SetLightColor` _btn_2_light (struct :`G` 1.0 :`A` 1.0) true)
      (`MaterialInstanceDynamic.SetVectorParameterValue` (`self.BTN_2_MAT`) "Color" (struct :`G` 1.0 :`A` 1.0)))
    (:`2`
      (`LightComponent.SetIntensity` _btn_3_light 5000.0)
      (`LightComponent.SetLightColor` _btn_3_light (struct :`G` 1.0 :`A` 1.0) true)
      (`MaterialInstanceDynamic.SetVectorParameterValue` (`self.BTN_3_MAT`) "Color" (struct :`G` 1.0 :`A` 1.0)))
    (:`3`
      (`LightComponent.SetIntensity` _btn_4_light 5000.0)
      (`LightComponent.SetLightColor` _btn_4_light (struct :`G` 1.0 :`A` 1.0) true)
      (`MaterialInstanceDynamic.SetVectorParameterValue` (`self.BTN_4_MAT`) "Color" (struct :`G` 1.0 :`A` 1.0)))))

(fn `CheckIfPuzzleIsComplete`
  (bind _outactors (`GameplayStatics.GetAllActorsOfClass` "/Game/Blueprints/BP_Placeable_Object.BP_Placeable_Object_C"))
  (for _array_element _outactors
    (set `self.isPuzzleComplete` (`/Game/Blueprints/BP_Placeable_Object.isPlacedOnCorrectSpot` _array_element)))
  (if (`self.isPuzzleComplete`)
    _))

(fn `DeactivateLights`
  (params (Lights :type Integer))
  (bind _btn_1_light (`self.Btn_1_Light`))
  (bind _btn_2_light (`self.Btn_2_Light`))
  (bind _btn_3_light (`self.Btn_3_Light`))
  (bind _btn_4_light (`self.Btn_4_Light`))
  (switch `int` Lights
    (:`0`
      (`LightComponent.SetIntensity` _btn_1_light 5000.0)
      (`LightComponent.SetLightColor` _btn_1_light (struct :`R` 1.0 :`A` 1.0) true)
      (`MaterialInstanceDynamic.SetVectorParameterValue` (`self.BTN_1_MAT`) "Color" (struct :`R` 1.0 :`A` 1.0)))
    (:`1`
      (`LightComponent.SetIntensity` _btn_2_light 5000.0)
      (`LightComponent.SetLightColor` _btn_2_light (struct :`R` 1.0 :`A` 1.0) true)
      (`MaterialInstanceDynamic.SetVectorParameterValue` (`self.BTN_2_MAT`) "Color" (struct :`R` 1.0 :`A` 1.0)))
    (:`2`
      (`LightComponent.SetIntensity` _btn_3_light 5000.0)
      (`LightComponent.SetLightColor` _btn_3_light (struct :`R` 1.0 :`A` 1.0) true)
      (`MaterialInstanceDynamic.SetVectorParameterValue` (`self.BTN_3_MAT`) "Color" (struct :`R` 1.0 :`A` 1.0)))
    (:`3`
      (`LightComponent.SetIntensity` _btn_4_light 5000.0)
      (`LightComponent.SetLightColor` _btn_4_light (struct :`R` 1.0 :`A` 1.0) true)
      (`MaterialInstanceDynamic.SetVectorParameterValue` (`self.BTN_4_MAT`) "Color" (struct :`R` 1.0 :`A` 1.0)))))

(fn `UserConstructionScript`
  (`|ExecutionSequence`
    (:`then_0`
      (bind _returnvalue (`PrimitiveComponent.CreateDynamicMaterialInstance` (`self.Button_01`) 0 "/Game/Materials/M_SimonButton.M_SimonButton"))
      (set `self.BTN_1_MAT` _returnvalue))
    (:`then_1`
      (bind _returnvalue_2 (`PrimitiveComponent.CreateDynamicMaterialInstance` (`self.Button_02`) 0 "/Game/Materials/M_SimonButton.M_SimonButton"))
      (set `self.BTN_2_MAT` _returnvalue_2))
    (:`then_2`
      (bind _returnvalue_3 (`PrimitiveComponent.CreateDynamicMaterialInstance` (`self.Button_03`) 0 "/Game/Materials/M_SimonButton.M_SimonButton"))
      (set `self.BTN_3_MAT` _returnvalue_3))
    (:`then_3`
      (bind _returnvalue_4 (`PrimitiveComponent.CreateDynamicMaterialInstance` (`self.Button_04`) 0 "/Game/Materials/M_SimonButton.M_SimonButton"))
      (set `self.BTN_4_MAT` _returnvalue_4))
    (:`then_4`
      (`self.DeactivateLights` 0)
      (`self.DeactivateLights` 1)
      (`self.DeactivateLights` 2)
      (`self.DeactivateLights` 3))))