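; Placeable oxygen tank piece, apparently for a puzzle, whose look is chosen by its Value variable.
; The construction script switches on Value to apply one of nine tank materials, varying in color and marking, to the static mesh's first slot.
; The event graph holds only disabled stub events, so the Blueprint runs no gameplay logic of its own.
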(fn `UserConstructionScript`
  (bind _staticmesh (`self.StaticMesh`))
  (switch `int` (`self.Value`)
    (:`0`
      (`PrimitiveComponent.SetMaterial` _staticmesh 0 "/Game/Models/OxygenTanksForPuzzle/Materials/OxygenTankPuzzle_PurpleRound1.OxygenTankPuzzle_PurpleRound1"))
    (:`1`
      (`PrimitiveComponent.SetMaterial` _staticmesh 0 "/Game/Models/OxygenTanksForPuzzle/Materials/OxygenTankPuzzle_PurpleRound2.OxygenTankPuzzle_PurpleRound2"))
    (:`2`
      (`PrimitiveComponent.SetMaterial` _staticmesh 0 "/Game/Models/OxygenTanksForPuzzle/Materials/OxygenTankPuzzle_PurpleDiamond2.OxygenTankPuzzle_PurpleDiamond2"))
    (:`3`
      (`PrimitiveComponent.SetMaterial` _staticmesh 0 "/Game/Models/OxygenTanksForPuzzle/Materials/OxygenTankPuzzle_PurpleDiamond3.OxygenTankPuzzle_PurpleDiamond3"))
    (:`4`
      (`PrimitiveComponent.SetMaterial` _staticmesh 0 "/Game/Models/OxygenTanksForPuzzle/Materials/OxygenTankPuzzle_Purple2.OxygenTankPuzzle_Purple2"))
    (:`5`
      (`PrimitiveComponent.SetMaterial` _staticmesh 0 "/Game/Models/OxygenTanksForPuzzle/Materials/OxygenTankPuzzle_GreenRound1.OxygenTankPuzzle_GreenRound1"))
    (:`6`
      (`PrimitiveComponent.SetMaterial` _staticmesh 0 "/Game/Models/OxygenTanksForPuzzle/Materials/OxygenTankPuzzle_GreenDiamond1.OxygenTankPuzzle_GreenDiamond1"))
    (:`7`
      (`PrimitiveComponent.SetMaterial` _staticmesh 0 "/Game/Models/OxygenTanksForPuzzle/Materials/OxygenTankPuzzle_Green2.OxygenTankPuzzle_Green2"))
    (:`8`
      (`PrimitiveComponent.SetMaterial` _staticmesh 0 "/Game/Models/OxygenTanksForPuzzle/Materials/OxygenTankPuzzle_Blue2.OxygenTankPuzzle_Blue2"))))