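; WeldArea is a trigger zone that swaps a set of old meshes for new ones when welded.
; A WeldGun entering the Box shows its welding particles and opens a Gate, which a one-second Delay then enters to perform the visibility swap.
; Leaving the Box hides the particles and closes the Gate, blocking the swap if the gun exits too early.
; The construction script keeps the new meshes hidden initially.
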(event `StartWelding`
  (`|ExecutionSequence`
    (:`then_0`
      (goto _label :!via `Open`))
    (:`then_1`
      (`KismetSystemLibrary.Delay` 1.0)
      (`/Engine/EditorBlueprintResources/StandardMacros.Gate` true :!label _label
        (:`Exit`
          (for _array_element (`self.OldMesh`)
            (`SceneComponent.SetVisibility` (`Actor.RootComponent` _array_element) false false))
          (for _array_element_2 (`self.NewMesh`)
            (`SceneComponent.SetVisibility` (`Actor.RootComponent` _array_element_2) true false)))))))

(event `StopWelding`
  (goto _label :!via `Close`))

(event `self.Box.OnComponentBeginOverlap`
  (params (OverlappedComponent :type "PrimitiveComponent Object Reference") (OtherActor :type "Actor Object Reference") (OtherComp :type "PrimitiveComponent Object Reference") (OtherBodyIndex :type Integer) (bFromSweep :type Boolean) (SweepResult :type "HitResult Structure (by ref)"))
  (bind _asweld_gun (cast `/Game/Blueprints/WeldGun` OtherActor))
  (`SceneComponent.SetVisibility` (`/Game/Blueprints/WeldGun.WeldingParticles` _asweld_gun) true false)
  (`self.StartWelding`))

(event `self.Box.OnComponentEndOverlap`
  (params (OverlappedComponent :type "PrimitiveComponent Object Reference") (OtherActor :type "Actor Object Reference") (OtherComp :type "PrimitiveComponent Object Reference") (OtherBodyIndex :type Integer))
  (bind _asweld_gun (cast `/Game/Blueprints/WeldGun` OtherActor))
  (`SceneComponent.SetVisibility` (`/Game/Blueprints/WeldGun.WeldingParticles` _asweld_gun) false false)
  (`self.StopWelding`))

(fn `UserConstructionScript`
  (for _array_element (`self.NewMesh`)
    (`SceneComponent.SetVisibility` (`Actor.RootComponent` _array_element) false false)))